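; Lobby player controller for a networked game, linking each player's lobby, chat and loading widgets to GM_Lobby.
; On BeginPlay it reads PlayerInfo from MyGameInstance, registers it, creates the UI and announces the player in chat.
; Events commented as server-side forward player updates to GM_Lobby or broadcast chat across its controller list, while client-side ones update widgets.
; Leaving destroys the session, then opens Map_Start on success.
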(event `self.ReceiveTick`
  (params (DeltaSeconds :type "Float (single-precision)")))

(event `Event_AddPlayerInfo`
  (params (PlayerInfo :type "/Game/NET/Game/Variable/Struct_Player_info Structure"))
  ;[1 1 1] 服务器，添加玩家信息
  (bind _asgm_lobby (cast `/Game/NET/Game/Lobby/GM_Lobby` (`GameplayStatics.GetGameMode`)))
  (`/Game/NET/Game/Lobby/GM_Lobby.Event_AddPlayerInfo` _asgm_lobby PlayerInfo))

(event `self.ReceiveBeginPlay`
  ;[1 1 1] 开始，初始化
  (`self.Event_Initialize`))

(event `Evant_ShowChatFrame`
  ;[1 1 1] 聊天
  ;;[1 1 1] 客户端，创建聊天框
  (bind _returnvalue (`|CreateWidget` "/Game/NET/UI/Chat/UI_LobbyChat.UI_LobbyChat_C" self))
  (bind _output_get (set `self.UI_ChatFrame` _returnvalue))
  (`UserWidget.AddToViewport` _output_get 0))

(event `Event_Initialize`
  ;[1 1 1] 客户端，初始化，从游戏实例中获取玩家信息
  (bind _asmy_game_instance (cast `/Game/NET/Game/MyGameInstance` (`GameplayStatics.GetGameInstance`)))
  (bind _output_get (set `self.PlayerInfo` (`/Game/NET/Game/MyGameInstance.PlayerInfo` _asmy_game_instance)))
  (`KismetSystemLibrary.PrintString` (`KismetTextLibrary.Conv_TextToString` (`.State_5_DBBEE8524B8DE1FD6A5B118C49B10C9D` (break `/Game/NET/Game/Variable/Struct_Player_info` _output_get))))
  ;[1 1 1] 添加人物信息、创建大厅UI
  (`self.Event_AddPlayerInfo` _output_get)
  (`self.Event_ShowLobbyUI`)
  ;[1 1 1] 聊天框初始化
  (`self.Evant_ShowChatFrame`)
  (`self.Event_AddChatInfo` "【系统】" (`|FormatText` "玩家{Name}进入了房间" (`.Name_4_9413B41E44B22CA1C444409AA13217EE` (break `/Game/NET/Game/Variable/Struct_Player_info` (`self.PlayerInfo`))))))

(event `Event_NewMessage`
  (params (Text :type Text))
  ;[1 1 1] 聊天
  ;;[1 1 1] 客户端，更新新的消息
  (`/Game/NET/UI/Chat/UI_Com_Chat.Event_UpDateNewInfo` (`/Game/NET/UI/Chat/UI_LobbyChat.UI_Com_ChatFrame` (`self.UI_ChatFrame`)) Text))

(event `Event_AddChatInfo`
  (params (before :type Text) (content :type Text))
  ;[1 1 1] 聊天
  ;;[1 1 1] 服务器，添加新的聊天信息
  (bind _asgm_lobby (cast `/Game/NET/Game/Lobby/GM_Lobby` (`GameplayStatics.GetGameMode`)))
  (for _array_element (`/Game/NET/Game/Lobby/GM_Lobby.PlayerControllerList` _asgm_lobby)
    (bind _aspc_lobby (cast `/Game/NET/Game/Lobby/PC_Lobby` _array_element))
    (`self.Event_NewMessage` _aspc_lobby (`|FormatText` "{before}：{content}" before content))))

(event `Event_ShowLobbyUI`
  ;[1 1 1] 客户端，创建显示大厅控件
  (set `self.bShowMouseCursor` true)
  (bind _returnvalue (`|CreateWidget` "/Game/NET/UI/UI_Lobby.UI_Lobby_C" self))
  (bind _output_get (set `self.UI_Lobby` _returnvalue))
  (`UserWidget.AddToViewport` _output_get 0)
  (`WidgetBlueprintLibrary.SetInputMode_GameAndUIEx` self (`self.UI_Lobby`))
  (`self.Event_UpDateAllPlayer`))

(event `Event_UpDateSelf`
  (params (PlayerInfo :type "Array of /Game/NET/Game/Variable/Struct_Player_info Structure") (CkptName :type Text) (MaxPlayerNumber :type Integer))
  (bind _ui_lobby (`self.UI_Lobby`))
  ;[1 1 1] 客户端，更新自身大厅控件信息
  (`/Game/NET/UI/UI_Lobby.Event_UpDateInfo` _ui_lobby PlayerInfo MaxPlayerNumber)
  (`/Game/NET/UI/UI_Lobby.Event_UpDateCkptName` _ui_lobby CkptName))

(event `Event_UpDateAllPlayer`
  ;[1 1 1] 服务器，更新所有玩家
  (bind _asgm_lobby (cast `/Game/NET/Game/Lobby/GM_Lobby` (`GameplayStatics.GetGameMode`)))
  (`/Game/NET/Game/Lobby/GM_Lobby.Event_UpDateAllPlayer` _asgm_lobby))

(event `Event_ShowLoading`
  ;[1 1 1] 客户端，创建加载页面
  (bind _returnvalue (`|CreateWidget` "/Game/NET/UI/UI_Loading.UI_Loading_C" self))
  (`UserWidget.AddToViewport` _returnvalue 0))

(event `Event_UpDatePlayerInfo`
  (params (Info :type "/Game/NET/Game/Variable/Struct_Player_info Structure"))
  ;[1 1 1] 服务器，更新玩家信息
  (bind _asgm_lobby (cast `/Game/NET/Game/Lobby/GM_Lobby` (`GameplayStatics.GetGameMode`)))
  (`/Game/NET/Game/Lobby/GM_Lobby.Event_UpDatePlayerInfo` _asgm_lobby Info))

(event `Event_LeaveRoom`
  ;[1 1 1] 客户端，离开房间
  (`DestroySessionCallbackProxy.DestroySession` self
    (:`OnSuccess`
      (`GameplayStatics.OpenLevel` "Map_Start"))))

(fn `UserConstructionScript`)