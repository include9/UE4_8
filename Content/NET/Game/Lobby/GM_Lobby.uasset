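; Lobby game mode that keeps the server-side room roster and starts the match by server travel.
; On BeginPlay it reads the checkpoint name and player cap from MyGameInstance.
; Logins are recorded and get a Lobby_Character spawned at the first PlayerStart found.
; Roster changes from logout, kicks or info updates (matched by player name) push the player list and room settings to every PC_Lobby controller.
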(event `self.K2_OnSwapPlayerControllers`
  (params (OldPC :type "PlayerController Object Reference") (NewPC :type "PlayerController Object Reference")))

(event `self.ReceiveBeginPlay`
  ;[1 1 1] 获取地图信息，保存到GAMEMOOD
  (`/Engine/EditorBlueprintResources/ActorMacros.Switch Has Authority`
    (:`Authority`
      (bind _asmy_game_instance (cast `/Game/NET/Game/MyGameInstance` (`GameplayStatics.GetGameInstance`)))
      (set `self.Ckpt_Name` (`/Game/NET/Game/MyGameInstance.CheckPointName` _asmy_game_instance))
      (set `self.MaxPlayerNumber` (`/Game/NET/Game/MyGameInstance.MaxPlayerNumber` _asmy_game_instance)))))

(event `self.K2_PostLogin`
  (params (NewPlayer :type "PlayerController Object Reference"))
  ;[1 1 1] 有玩家登入时
  (`/Engine/EditorBlueprintResources/ActorMacros.Switch Has Authority`
    (:`Authority`
      (`KismetArrayLibrary.Array_AddUnique` (`self.PlayerControllerList`) NewPlayer)
      (`self.Event_PawnPlayer` NewPlayer))))

(event `self.K2_OnLogout`
  (params (ExitingController :type "Controller Object Reference"))
  ;[1 1 1] 玩家登出
  (`/Engine/EditorBlueprintResources/ActorMacros.Switch Has Authority`
    (:`Authority`
      (for (_array_element _array_index) (`self.PlayerControllerList`)
        (if (== _array_element ExitingController)
          (`KismetArrayLibrary.Array_RemoveItem` (`self.PlayerControllerList`) _array_element)
          (`KismetArrayLibrary.Array_Remove` (`self.PlayerInfoList`) _array_index)))
      ;[1 1 1] 不是房主，实验
      (`self.Event_UpDateAllPlayer`))))

(event `Event_PawnPlayer`
  (params (PC :type "PlayerController Object Reference"))
  (bind _returnvalue (`Controller.K2_GetPawn` PC))
  ;[1 1 1] 服务器，生成玩家
  (`/Engine/EditorBlueprintResources/StandardMacros.IsValid` _returnvalue
    (:`Is Valid`
      (`self.K2_DestroyActor` _returnvalue))
    (:`Is Not Valid`
      _))
  ;;[1 1 1] 嘤嘤嘤
  (bind _outactors (`GameplayStatics.GetAllActorsOfClass` "/Script/Engine.PlayerStart"))
  (bind _returnvalue_2 (`|SpawnActorFromClass` "/Game/NET/Game/Lobby/Lobby_Character.Lobby_Character_C" (`KismetMathLibrary.MakeTransform` (`self.K2_GetActorLocation` (`|GetArrayItem` _outactors))) "AdjustIfPossibleButAlwaysSpawn" "OverrideRootScale" null null))
  (`Controller.Possess` PC _returnvalue_2))

(event `Event_AddPlayerInfo`
  (params (APlayerInfo :type "/Game/NET/Game/Variable/Struct_Player_info Structure (by ref)"))
  ;[1 1 1] 服务器，添加玩家信息
  (`KismetArrayLibrary.Array_Add` (`self.PlayerInfoList`) APlayerInfo))

(event `Event_KickPlayer`
  (params (index :type Integer))
  ;[1 1 1] 服务器，踢出玩家
  (bind _aspc_lobby (cast `/Game/NET/Game/Lobby/PC_Lobby` (`|GetArrayItem` (`self.PlayerControllerList`) index)))
  (`/Game/NET/Game/Lobby/PC_Lobby.Event_LeaveRoom` _aspc_lobby)
  (`self.Event_UpDateAllPlayer`))

(event `Event_UpDateAllPlayer`
  ;[1 1 1] 服务器，更新所有玩家
  (for _array_element (`self.PlayerControllerList`)
    (bind _aspc_lobby (cast `/Game/NET/Game/Lobby/PC_Lobby` _array_element))
    (`/Game/NET/Game/Lobby/PC_Lobby.Event_UpDateSelf` _aspc_lobby (`self.PlayerInfoList`) (`self.Ckpt_Name`) (`self.MaxPlayerNumber`))))

(event `Event_Start`
  (params (B :type String))
  ;[1 1 1] 场景漫游
  (`KismetSystemLibrary.ExecuteConsoleCommand` (`KismetStringLibrary.Concat_StrStr` "ServerTravel " B) (`GameplayStatics.GetPlayerController` 0)))

(event `Event_UpDatePlayerInfo`
  (params (Info :type "/Game/NET/Game/Variable/Struct_Player_info Structure"))
  ;[1 1 1] 服务器，更新玩家属性
  (`KismetArrayLibrary.Array_Clear` (`self.NewPlayerInfoList`))
  (for _array_element (`self.PlayerInfoList`)
    (if (`KismetTextLibrary.EqualEqual_TextText` (`.Name_4_9413B41E44B22CA1C444409AA13217EE` (break `/Game/NET/Game/Variable/Struct_Player_info` _array_element)) (`.Name_4_9413B41E44B22CA1C444409AA13217EE` (break `/Game/NET/Game/Variable/Struct_Player_info` Info)))
      (`KismetArrayLibrary.Array_Add` (`self.NewPlayerInfoList`) Info)
      (else
        (`KismetArrayLibrary.Array_Add` (`self.NewPlayerInfoList`) _array_element))))
  (set `self.PlayerInfoList` (`self.NewPlayerInfoList`))
  (`self.Event_UpDateAllPlayer`))

(fn `UserConstructionScript`)