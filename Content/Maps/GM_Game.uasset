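; Game mode for the game map that spawns and possesses a player character on the server when player controllers are swapped.
; OnSwapPlayerControllers passes the old controller to a spawn event, which destroys that controller's current pawn.
; It then spawns a Lobby_Character at the first PlayerStart found, adjusting for collisions but always spawning, and has that controller possess it.
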(event `self.ReceiveBeginPlay`)

(event `self.K2_OnSwapPlayerControllers`
  (params (OldPC :type "PlayerController Object Reference") (NewPC :type "PlayerController Object Reference"))
  (`self.Event_PawnPlayer` OldPC))

(event `Event_PawnPlayer`
  (params (PC :type "PlayerController Object Reference"))
  (bind _returnvalue (`Controller.K2_GetPawn` PC))
  ;[1 1 1] 服务器，生成玩家
  (`/Engine/EditorBlueprintResources/StandardMacros.IsValid` _returnvalue
    (:`Is Valid`
      (`self.K2_DestroyActor` _returnvalue))
    (:`Is Not Valid`
      _))
  ;;[1 1 1] 嘤嘤嘤
  (bind _outactors (`GameplayStatics.GetAllActorsOfClass` "/Script/Engine.PlayerStart"))
  (bind _returnvalue_2 (`|SpawnActorFromClass` "/Game/NET/Game/Lobby/Lobby_Character.Lobby_Character_C" (`KismetMathLibrary.MakeTransform` (`self.K2_GetActorLocation` (`|GetArrayItem` _outactors))) "AdjustIfPossibleButAlwaysSpawn" "OverrideRootScale" null null))
  (`Controller.Possess` PC _returnvalue_2))

(fn `UserConstructionScript`)