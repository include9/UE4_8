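; In-match player controller for a session-based multiplayer game, creating the game HUD and tracking the player's kills and deaths.
; Name comes from the GameInstance; stat changes update the HUD and GameMode's per-index info array, while respawns route through GameMode.
; Leaving at index 0 takes the owner room-teardown path; others save match info to the GameInstance, destroy the session and open the "Jiesuan" (settlement) level.
; Number keys directly trigger kill, death and respawn.
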(event `self.ReceiveBeginPlay`
  (`self.Init`))

(event `Init`
  (bind _index (`self.index`))
  ;[1 1 1] 初始化
  (bind _name (`self.getPlayerName`))
  (bind _output_get (set `self.Name` _name))
  (bind _returnvalue (`|CreateWidget` "/Game/Game/UI_Game.UI_Game_C" null _output_get))
  (bind _output_get_2 (set `self.UI_Game` _returnvalue))
  (`UserWidget.AddToViewport` _output_get_2 0)
  (`self.SETInfoByIndex` _index (make `/Game/Game/Game_PlayerInfo` _index _output_get))
  (`self.relife`))

(event `Key|M`
  (params (Key :type "Key Structure"))
  ;[1 1 1] 按下菜单键
  (:`Pressed`
    (`/Game/Game/UI_Game.Event_OnClickMenu` (`self.UI_Game`))))

(event `Key|Eight`
  (params (Key :type "Key Structure")))

(event `Key|Zero`
  (params (Key :type "Key Structure"))
  (:`Pressed`
    (`self.KillillAnEneny`)))

(event `Key|One`
  (params (Key :type "Key Structure"))
  (:`Pressed`
    (`self.BeenKilled`)))

(event `Key|Nine`
  (params (Key :type "Key Structure"))
  (:`Pressed`
    (`self.relife`)))

(event `setIndex`
  (params (index :type Integer))
  ;[1 1 1] 设置Index
  (set `self.index` index))

(event `SetPlayetInfo`
  (params (GameInfoArray :type "Array of /Game/Game/Game_PlayerInfo Structure"))
  ;[1 1 1] 设置本地PlayerInfo
  (set `self.GameInfoArray` GameInfoArray))

(event `SETInfoByIndex`
  (params (Index :type Integer) (Item :type "/Game/Game/Game_PlayerInfo Structure (by ref)"))
  ;[1 1 1] 通过index设置Gaemode的Info数组
  (bind _asgame_mode_game (cast `/Game/Game/GameMode_Game` (`GameplayStatics.GetGameMode`)))
  (`/Game/Game/GameMode_Game.SETInfoByIndex` _asgame_mode_game Index Item))

(event `reLifeServer`
  (params (PC :type "PlayerController Object Reference") (index :type Integer))
  ;[1 1 1] 重生
  (bind _asgame_mode_game (cast `/Game/Game/GameMode_Game` (`GameplayStatics.GetGameMode`)))
  (`/Game/Game/GameMode_Game.Event_PawnPlayer` _asgame_mode_game PC index))

(event `relife`
  ;[1 1 1] 重生
  (`self.reLifeServer` self self (`self.index`)))

(event `LeaveRoom`
  ;[1 1 1] （通用）离开房间,复制信息到instance
  (if (== (`self.index`) 0)
    (`self.LeaveRoom_Owner`)
    (else
      (`self.EventLeave`))))

(event `EventLeave`
  ;[1 1 1] 离开房间
  (bind _asmy_game_instance (cast `/Game/NET/Game/MyGameInstance` (`GameplayStatics.GetGameInstance`)))
  (set `/Game/NET/Game/MyGameInstance.GameInfoArray` (`self.GameInfoArray`) _asmy_game_instance)
  (`DestroySessionCallbackProxy.DestroySession` self
    (:`then`
      (`GameplayStatics.OpenLevel` "Jiesuan"))))

(event `UpdateKDA`
  (bind _index (`self.index`))
  (bind _ui_game (`self.UI_Game`))
  ;[1 1 1] 更新KDA
  (set `/Game/Game/UI_Game.KillNumber` (`self.Kill`) _ui_game)
  (set `/Game/Game/UI_Game.DeathNumber` (`self.Death`) _ui_game)
  (`self.SETInfoByIndex` _index (make `/Game/Game/Game_PlayerInfo` _index (`self.Name`) (`self.Kill`) (`self.Death`))))

(event `LeaveRoom_Owner`
  ;[1 1 1] 调用GameMode::DeatroyRoom
  (bind _asgame_mode_game (cast `/Game/Game/GameMode_Game` (`GameplayStatics.GetGameMode`)))
  (`/Game/Game/GameMode_Game.DestroyRoom` _asgame_mode_game))

(event `KillillAnEneny`
  (bind _index (`self.index`))
  ;[1 1 1] 击杀++
  (bind _output_get (set `self.Kill` (+ (`self.Kill`) 1)))
  (set `/Game/Game/UI_Game.KillNumber` _output_get (`self.UI_Game`))
  (`self.SETInfoByIndex` _index (make `/Game/Game/Game_PlayerInfo` _index (`self.Name`) (`self.Kill`) (`self.Death`))))

(event `BeenKilled`
  (bind _index (`self.index`))
  ;[1 1 1] 死亡++
  (bind _output_get (set `self.Death` (+ (`self.Death`) 1)))
  (set `/Game/Game/UI_Game.DeathNumber` _output_get (`self.UI_Game`))
  (`self.SETInfoByIndex` _index (make `/Game/Game/Game_PlayerInfo` _index (`self.Name`) (`self.Kill`) (`self.Death`))))

(fn `getPlayerName`
  (returns (Name :type Text))
  (bind _asmy_game_instance (cast `/Game/NET/Game/MyGameInstance` (`GameplayStatics.GetGameInstance`)))
  (return (`.Name_4_9413B41E44B22CA1C444409AA13217EE` (break `/Game/NET/Game/Variable/Struct_Player_info` (`/Game/NET/Game/MyGameInstance.PlayerInfo` _asmy_game_instance)))))

(fn `UserConstructionScript`)